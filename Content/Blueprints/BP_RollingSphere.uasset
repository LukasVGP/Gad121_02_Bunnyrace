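; BP_RollingSphere is a hazard for the vehicle game that starts moving when a vehicle pawn first overlaps the actor.
; That overlap latches a trigger and stores the actor's forward vector, which Tick uses to translate it at RollSpeed without sweeping or rotating.
; A vehicle pawn overlapping the sphere mesh makes the game mode deduct a life, then gets destroyed.
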(event Custom|OnComponentBeginOverlap_Event
  (params (OverlappedComponent :type Primitive%20Component%20Object%20Reference) (OtherActor :type Actor%20Object%20Reference) (OtherComp :type Primitive%20Component%20Object%20Reference) (OtherBodyIndex :type Integer) (bFromSweep :type Boolean) (SweepResult :type Hit%20Result%20Structure%20%28by%20ref%29))
  (bind _asbp_vehicle_adv_pawn_base (Utilities|Casting|CastToBP_VehicleAdvPawnBase OtherActor))
  (bind _asbp_vehicle_adv_game_mode (Utilities|Casting|CastToBP_VehicleAdvGameMode (Game|GetGameMode)))
  (Default|LoseLife _asbp_vehicle_adv_game_mode)
  (Actor|DestroyActor _asbp_vehicle_adv_pawn_base))

(event EventBeginPlay
  (Collision|AssignOnComponentBeginOverlap (Variables|Default|GetSphereMesh) (delegate Custom|OnComponentBeginOverlap_Event)))

(event Collision|EventActorBeginOverlap
  (params (OtherActor :type Actor%20Object%20Reference))
  (Utilities|Casting|CastToBP_VehicleAdvPawnBase OtherActor)
  (if (not (Variables|Default|GetbTriggered))
    (Variables|Default|SetbTriggered true)
    (Variables|Default|SetRollDirection (Transformation|GetActorForwardVector))))

(event EventTick
  (params (DeltaSeconds :type Float%20%28single-precision%29))
  (if (Variables|Default|GetbTriggered)
    (Transformation|AddActorWorldOffset (* (* (Variables|Default|GetRollDirection) (Variables|Default|GetRollSpeed)) DeltaSeconds))))

(fn ConstructionScript)