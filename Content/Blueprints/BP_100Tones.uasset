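; BP_100Tones is a heavy-weight trap that destroys player vehicles and costs a life on contact.
; Tick cycles WeightMesh between its starting Z and a raised height with separate rise and fall speeds, flipping Triggered at each end.
; A vehicle overlapping the actor can force a fall and schedule a delayed ResetTrap that snaps the weight back to start.
; Mesh overlap and actor Hit both call LoseLife on the game mode.
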(event Custom|OnComponentBeginOverlap_Event
  (params (OverlappedComponent :type Primitive%20Component%20Object%20Reference) (OtherActor :type Actor%20Object%20Reference) (OtherComp :type Primitive%20Component%20Object%20Reference) (OtherBodyIndex :type Integer) (bFromSweep :type Boolean) (SweepResult :type Hit%20Result%20Structure%20%28by%20ref%29))
  (bind _asbp_vehicle_adv_pawn_base (Utilities|Casting|CastToBP_VehicleAdvPawnBase OtherActor))
  (bind _asbp_vehicle_adv_game_mode (Utilities|Casting|CastToBP_VehicleAdvGameMode (Game|GetGameMode)))
  (Default|LoseLife _asbp_vehicle_adv_game_mode)
  (Actor|DestroyActor _asbp_vehicle_adv_pawn_base))

(event Custom|ResetTrap
  (bind _weightmesh (Variables|Default|GetWeightMesh))
  (bind _relativelocation (Variables|/Script/Engine.SceneComponent|GetRelativeLocation _weightmesh))
  (bind (_x _y _z) (Math|Vector|BreakVector _relativelocation))
  (Variables|Default|SetbTriggered false)
  (Transformation|SetRelativeLocation (Variables|Default|GetWeightMesh) (Math|Vector|MakeVector _x _y (Math|Conversions|ToFloat(Integer) (Variables|Default|GetSpawnZ))) false false))

(event EventBeginPlay
  (Variables|Default|SetSpawnZ (Math|Float|Truncate (.Z (Math|Vector|BreakVector (Variables|/Script/Engine.SceneComponent|GetRelativeLocation (Variables|Default|GetWeightMesh))))))
  (Collision|AssignOnComponentBeginOverlap (Variables|Default|GetWeightMesh) (delegate Custom|OnComponentBeginOverlap_Event)))

(event Collision|EventActorBeginOverlap
  (params (OtherActor :type Actor%20Object%20Reference))
  (Utilities|Casting|CastToBP_VehicleAdvPawnBase OtherActor)
  (if (not (Variables|Default|GetbTriggered))
    (Variables|Default|SetbTriggered true)
    (Utilities|Time|SetTimerbyFunctionName self "ResetTrap" 2e+01)))

(event EventTick
  (params (DeltaSeconds :type Float%20%28single-precision%29))
  (bind _weightmesh (Variables|Default|GetWeightMesh))
  (bind _weightmesh_2 (Variables|Default|GetWeightMesh))
  (bind _relativelocation (Variables|/Script/Engine.SceneComponent|GetRelativeLocation _weightmesh_2))
  (bind _relativelocation_2 (Variables|/Script/Engine.SceneComponent|GetRelativeLocation _weightmesh))
  (bind (_x _y _z) (Math|Vector|BreakVector _relativelocation))
  (bind (_x_2 _y_2 _z_2) (Math|Vector|BreakVector _relativelocation_2))
  (if (Variables|Default|GetbTriggered)
    (Transformation|SetRelativeLocation (Variables|Default|GetWeightMesh) (Math|Vector|MakeVector _x_2 _y_2 (Math|Float|Max(Float) (- _z_2 (* DeltaSeconds (Variables|Default|GetFallSpeed))) (Math|Conversions|ToFloat(Integer) (Variables|Default|GetSpawnZ)))) false false)
    (if (<= (.Z (Math|Vector|BreakVector (Variables|/Script/Engine.SceneComponent|GetRelativeLocation (Variables|Default|GetWeightMesh)))) (Math|Conversions|ToFloat(Integer) (Variables|Default|GetSpawnZ)))
      (Variables|Default|SetbTriggered false))
    (else
      (Transformation|SetRelativeLocation (Variables|Default|GetWeightMesh) (Math|Vector|MakeVector _x _y (Math|Float|Min(Float) (+ _z (* (Variables|Default|GetRiseSpeed) DeltaSeconds)) (+ (Variables|Default|GetSpawnZ) (Variables|Default|GetHeightAboveTrigger)))) false false)
      (if (>= (.Z (Math|Vector|BreakVector (Variables|/Script/Engine.SceneComponent|GetRelativeLocation (Variables|Default|GetWeightMesh)))) (+ (Variables|Default|GetSpawnZ) (Variables|Default|GetHeightAboveTrigger)))
        (Variables|Default|SetbTriggered true)))))

(event Collision|EventHit
  (params (MyComp :type Primitive%20Component%20Object%20Reference) (Other :type Actor%20Object%20Reference) (OtherComp :type Primitive%20Component%20Object%20Reference) (bSelfMoved :type Boolean) (HitLocation :type Vector :default "0, 0, 0") (HitNormal :type Vector :default "0, 0, 0") (NormalImpulse :type Vector :default "0, 0, 0") (Hit :type Hit%20Result%20Structure%20%28by%20ref%29))
  (bind _asbp_vehicle_adv_pawn_base (Utilities|Casting|CastToBP_VehicleAdvPawnBase Other))
  (bind _asbp_vehicle_adv_game_mode (Utilities|Casting|CastToBP_VehicleAdvGameMode (Game|GetGameMode)))
  (Default|LoseLife _asbp_vehicle_adv_game_mode)
  (Actor|DestroyActor _asbp_vehicle_adv_pawn_base))

(fn ConstructionScript)