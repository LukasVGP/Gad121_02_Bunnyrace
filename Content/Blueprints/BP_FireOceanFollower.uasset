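; BP_FireOceanFollower is a hazard actor that acts as a kill plane beneath the player's vehicle.
; Every tick it moves to the player pawn's X and Y at a fixed FollowDepth height.
; When an unattached vehicle pawn overlaps it, the game mode deducts a life and, unless the game is over, the vehicle respawns at its checkpoint.
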(event EventBeginPlay)

(event Collision|EventActorBeginOverlap
  (params (OtherActor :type Actor%20Object%20Reference))
  (bind _asbp_vehicle_adv_pawn_base (Utilities|Casting|CastToBP_VehicleAdvPawnBase OtherActor))
  (if (not (Utilities|IsValid (Actor|GetAttachParentActor _asbp_vehicle_adv_pawn_base)))
    (bind _asbp_vehicle_adv_game_mode (Utilities|Casting|CastToBP_VehicleAdvGameMode (Game|GetGameMode)))
    (Default|LoseLife _asbp_vehicle_adv_game_mode)
    (if (not (Variables|/Game/VehicleTemplate/Blueprints/BP_VehicleAdvGameMode.BP_VehicleAdvGameMode_C|GetbGameOver _asbp_vehicle_adv_game_mode))
      (Default|RespawnatCheckpoint _asbp_vehicle_adv_pawn_base))))

(event EventTick
  (params (DeltaSeconds :type Float%20%28single-precision%29))
  (bind _returnvalue (Game|Player|GetPlayerPawn 0))
  (bind _returnvalue_2 (Transformation|GetActorLocation _returnvalue))
  (bind (_x _y) (Math|Vector|BreakVector _returnvalue_2))
  (Transformation|SetActorLocation (Math|Vector|MakeVector _x _y (Variables|Default|GetFollowDepth)) false false))

(fn ConstructionScript)