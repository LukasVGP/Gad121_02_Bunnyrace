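; BP_FireWall is a hazard for a vehicle game that advances along its forward vector and triggers a loss through the game mode when it overlaps the player's vehicle pawn class.
; While active, Tick moves it at a set speed and flickers its light with a sine wave.
; BeginPlay registers it with the game mode and, after a short delay, measures its distance to the player, which RespawnBehindPlayer reuses to teleport it behind them.
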(event Custom|RespawnBehindPlayer
  (bind _returnvalue (Game|Player|GetPlayerPawn 0))
  (Transformation|SetActorLocation (+ (Transformation|GetActorLocation _returnvalue) (* (Transformation|GetActorForwardVector _returnvalue) (* (Variables|Default|GetInitialFireWallDistance) -1.0))) false true))

(event Custom|MeasureInitialDistance
  (Variables|Default|SetInitialFireWallDistance (Transformation|GetDistanceTo (Game|Player|GetPlayerPawn 0))))

(event EventBeginPlay
  (bind _self self)
  (bind _asbp_vehicle_adv_game_mode (Utilities|Casting|CastToBP_VehicleAdvGameMode (Game|GetGameMode)))
  (Variables|/Game/VehicleTemplate/Blueprints/BP_VehicleAdvGameMode.BP_VehicleAdvGameMode_C|SetFireWallRef _asbp_vehicle_adv_game_mode _self)
  (Utilities|Time|SetTimerbyFunctionName _self "MeasureInitialDistance" 0.5))

(event Collision|EventActorBeginOverlap
  (params (OtherActor :type Actor%20Object%20Reference))
  (bind _asbp_vehicle_adv_pawn_base (Utilities|Casting|CastToBP_VehicleAdvPawnBase OtherActor))
  (bind _asbp_vehicle_adv_game_mode (Utilities|Casting|CastToBP_VehicleAdvGameMode (Game|GetGameMode)))
  (Default|TriggerLose _asbp_vehicle_adv_game_mode))

(event EventTick
  (params (DeltaSeconds :type Float%20%28single-precision%29))
  (if (Variables|FireWall|GetbFireWallActive)
    (Transformation|AddActorWorldOffset (* (* (Transformation|GetActorForwardVector) (Variables|FireWall|GetFireWallSpeed)) DeltaSeconds))
    (bind _output_get (Variables|Default|SetTimeAccumulator (+ (Variables|Default|GetTimeAccumulator) DeltaSeconds)))
    (Rendering|Components|Light|SetIntensity (Variables|Default|GetFireLight) (+ (* (Math|Trig|Sin(Radians) (* _output_get (Variables|Default|GetFlickerSpeed))) 2e+03) (Variables|Default|GetBaseLightIntensity)))))

(fn ConstructionScript)