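; Fire pillar hazard that ignites when a vehicle pawn enters its trigger and costs the player a life on contact with the fire.
; Activation switches on its components and glow light, then a timer switches them off after ActiveDuration.
; While active, vehicles in FireBase call LoseLife on the game mode from activation, overlap and Tick checks; only Tick destroys the pawn.
; Cooldown reactivation timers are present but unconnected.
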(event Custom|ActivatePillar
  (Variables|Default|SetbIsActive true)
  (for _array_element (Actor|GetComponentsByClass "/Script/Engine.ActorComponent")
    (Components|Activation|Activate _array_element true))
  (Rendering|Components|Light|SetIntensity (Variables|Default|GetFireGlow) 6e+03)
  (Utilities|Time|SetTimerbyFunctionName self "DeactivatePillar" (Variables|Default|GetActiveDuration))
  (for _array_element_2 (Collision|GetOverlappingActors (Variables|Default|GetFireBase) 0 :!class /Script/Engine.PrimitiveComponent)
    (Utilities|Casting|CastToBP_VehicleAdvPawnBase _array_element_2)
    (bind _asbp_vehicle_adv_game_mode (Utilities|Casting|CastToBP_VehicleAdvGameMode (Game|GetGameMode)))
    (Default|LoseLife _asbp_vehicle_adv_game_mode)))

(event Custom|DeactivatePillar
  (Variables|Default|SetbIsActive false)
  (for _array_element (Actor|GetComponentsByClass "/Script/Engine.ActorComponent")
    (Components|Activation|Deactivate _array_element))
  (Rendering|Components|Light|SetIntensity (Variables|Default|GetFireGlow) 0.0))

(event Custom|OnTriggerEntered
  (params (OverlappedComponent :type Primitive%20Component%20Object%20Reference) (OtherActor :type Actor%20Object%20Reference) (OtherComp :type Primitive%20Component%20Object%20Reference) (OtherBodyIndex :type Integer) (bFromSweep :type Boolean) (SweepResult :type Hit%20Result%20Structure%20%28by%20ref%29))
  (Utilities|Casting|CastToBP_VehicleAdvPawnBase OtherActor)
  (if (not (Variables|Default|GetbIsActive))
    (CallFunction|ActivatePillar)))

(event Custom|OnFireBaseOverlap
  (params (OverlappedComponent :type Primitive%20Component%20Object%20Reference) (OtherActor :type Actor%20Object%20Reference) (OtherComp :type Primitive%20Component%20Object%20Reference) (OtherBodyIndex :type Integer) (bFromSweep :type Boolean) (SweepResult :type Hit%20Result%20Structure%20%28by%20ref%29))
  (if (Variables|Default|GetbIsActive)
    (Utilities|Casting|CastToBP_VehicleAdvPawnBase OtherActor)
    (bind _asbp_vehicle_adv_game_mode (Utilities|Casting|CastToBP_VehicleAdvGameMode (Game|GetGameMode)))
    (Default|LoseLife _asbp_vehicle_adv_game_mode)))

(event EventBeginPlay
  (Collision|AssignOnComponentBeginOverlap (Variables|Default|GetTrigger) (delegate Custom|OnTriggerEntered))
  (Collision|AssignOnComponentBeginOverlap (Variables|Default|GetFireBase) (delegate Custom|OnFireBaseOverlap)))

(event Collision|EventActorBeginOverlap
  (params (OtherActor :type Actor%20Object%20Reference)))

(event EventTick
  (params (DeltaSeconds :type Float%20%28single-precision%29))
  (if (Variables|Default|GetbIsActive)
    (for _array_element (Collision|GetOverlappingActors (Variables|Default|GetFireBase) 0 :!class /Script/Engine.PrimitiveComponent)
      (bind _asbp_vehicle_adv_pawn_base (Utilities|Casting|CastToBP_VehicleAdvPawnBase _array_element))
      (bind _asbp_vehicle_adv_game_mode (Utilities|Casting|CastToBP_VehicleAdvGameMode (Game|GetGameMode)))
      (Default|LoseLife _asbp_vehicle_adv_game_mode)
      (Actor|DestroyActor _asbp_vehicle_adv_pawn_base))))

(fn ConstructionScript)