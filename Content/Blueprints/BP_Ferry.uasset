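; One-way car ferry that carries the player's vehicle from point A to point B once the game mode's coin requirement is met.
; Overlapping it docks the vehicle and runs a timer-driven HUD countdown before departure.
; Tick moves the ferry, pinning the vehicle by stored offset and zeroed velocities rather than attachment.
; On arrival it disables ferry collision, teleports the vehicle to the exit point and wakes its physics.
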(event Custom|ShowFerryMsg
  (params (Msg :type Text))
  (bind _asbp_vehicle_adv_player_controller (Utilities|Casting|CastToBP_VehicleAdvPlayerController (Game|GetPlayerController 0)))
  (Default|ShowFerryMessage (Variables|/Game/VehicleTemplate/Blueprints/BP_VehicleAdvPlayerController.BP_VehicleAdvPlayerController_C|GetVehicleHud _asbp_vehicle_adv_player_controller) Msg))

(event Custom|HideFerryMsg
  (bind _asbp_vehicle_adv_player_controller (Utilities|Casting|CastToBP_VehicleAdvPlayerController (Game|GetPlayerController 0)))
  (Default|HideFerryMessage (Variables|/Game/VehicleTemplate/Blueprints/BP_VehicleAdvPlayerController.BP_VehicleAdvPlayerController_C|GetVehicleHud _asbp_vehicle_adv_player_controller)))

(event Custom|FerryCount3
  (CallFunction|ShowFerryMsg (Utilities|Text|MakeLiteralText "Stay put! The car ferry starts in 3"))
  (Utilities|Time|SetTimerbyFunctionName self "FerryCount2" 1.0))

(event Custom|FerryCount2
  (CallFunction|ShowFerryMsg (Utilities|Text|MakeLiteralText "Stay put! The car ferry starts in 2"))
  (Utilities|Time|SetTimerbyFunctionName self "FerryCount1" 1.0))

(event Custom|FerryCount1
  (CallFunction|ShowFerryMsg (Utilities|Text|MakeLiteralText "Stay put! The car ferry starts in 1"))
  (Utilities|Time|SetTimerbyFunctionName self "StartFerry" 1.0))

(event Custom|StartFerry
  (CallFunction|HideFerryMsg)
  (Variables|Default|SetbActivated true))

(event EventBeginPlay
  (bind _pointaref (Variables|Default|GetPointARef))
  (Utilities|IsValid _pointaref
    (:Is%20Valid
      (Transformation|SetActorLocation (Transformation|GetActorLocation _pointaref) false true))))

(event Collision|EventActorBeginOverlap
  (params (OtherActor :type Actor%20Object%20Reference))
  (Utilities|Casting|CastToBP_VehicleAdvPawnBase OtherActor)
  (if (not (or (or (Variables|Default|GetbActivated) (Variables|Default|GetbAtB)) (Variables|Default|GetbPlayerDocked)))
    (if (Variables|Default|GetbCoinsPaid)
      (bind _output_get (Variables|Default|SetDockedVehicle OtherActor :!label _label))
      (Variables|Default|SetDockOffset (- (Transformation|GetActorLocation _output_get) (Transformation|GetActorLocation)))
      (Variables|Default|SetbPlayerDocked true)
      (Rendering|SetVisibility (Variables|Default|GetRedCube) false false)
      (CallFunction|FerryCount3)
      (else
        (bind _asbp_vehicle_adv_game_mode (Utilities|Casting|CastToBP_VehicleAdvGameMode (Game|GetGameMode)))
        (if (>= (Variables|/Game/VehicleTemplate/Blueprints/BP_VehicleAdvGameMode.BP_VehicleAdvGameMode_C|GetCoinCount _asbp_vehicle_adv_game_mode) (Variables|Default|GetRequiredCoins))
          (goto _label)
          (else
            (CallFunction|ShowFerryMsg (Utilities|Text|MakeLiteralText "Not enough coins go back, you need 30 coins!"))
            (Utilities|Time|SetTimerbyFunctionName self "HideFerryMsg" 3.0)))))))

(event EventTick
  (params (DeltaSeconds :type Float%20%28single-precision%29))
  (bind _returnvalue (Transformation|GetActorLocation))
  (bind _dockedvehicle (Variables|Default|GetDockedVehicle))
  (bind _pointbref (Variables|Default|GetPointBRef))
  (bind _returnvalue_2 (Transformation|GetActorLocation _pointbref))
  (if (Variables|Default|GetbActivated)
    (if (<= (Math|Vector|VectorLength (- _returnvalue _returnvalue_2)) 5e+01)
      (Transformation|SetActorLocation _returnvalue_2 false true)
      (Variables|Default|SetbActivated false)
      (Variables|Default|SetbAtB true)
      (if (Variables|Default|GetbPlayerDocked)
        (Transformation|DetachFromActor (Variables|Default|GetDockedVehicle) "KeepWorld" "KeepWorld" "KeepWorld")
        (Collision|SetCollisionEnabled (Variables|Default|GetFerryMesh) "NoCollision")
        (Utilities|FlowControl|Delay 0.1)
        (Transformation|SetActorLocation (Variables|Default|GetDockedVehicle) (Transformation|GetActorLocation (Variables|Default|GetFerryEndPointSpawn)) false true)
        (bind _asbp_vehicle_adv_pawn_base (Utilities|Casting|CastToBP_VehicleAdvPawnBase (Variables|Default|GetDockedVehicle)))
        (Physics|SetSimulatePhysics (Variables|/Script/ChaosVehicles.WheeledVehiclePawn|GetMesh _asbp_vehicle_adv_pawn_base) true)
        (Class|PrimitiveComponent|WakeRigidBody (Variables|/Script/ChaosVehicles.WheeledVehiclePawn|GetMesh _asbp_vehicle_adv_pawn_base) "None")
        (Physics|SetPhysicsLinearVelocity (Variables|/Script/ChaosVehicles.WheeledVehiclePawn|GetMesh _asbp_vehicle_adv_pawn_base) "0.000000, 0.000000, -400.000000" false "None")
        (Class|PrimitiveComponent|SetPhysicsAngularVelocityinDegrees (Variables|/Script/ChaosVehicles.WheeledVehiclePawn|GetMesh _asbp_vehicle_adv_pawn_base) "0, 0, 0" false "None")
        (Variables|Default|SetbPlayerDocked false)
        (CallFunction|ShowFerryMsg (Utilities|Text|MakeLiteralText "Ok you can drive on"))
        (Utilities|Time|SetTimerbyFunctionName self "HideFerryMsg" 5.0))
      (else
        (Transformation|SetActorLocation (+ _returnvalue (* (Math|Vector|GetUnitDirection(Vector) _returnvalue _returnvalue_2) (Math|Conversions|ToVector(Float) (* (Math|Conversions|ToFloat(Integer) (Variables|Default|GetFerrySpeed)) DeltaSeconds)))) false false)
        (if (Variables|Default|GetbPlayerDocked)
          (Transformation|SetActorLocation _dockedvehicle (+ (Transformation|GetActorLocation) (Variables|Default|GetDockOffset)) false true)
          (bind _asbp_vehicle_adv_pawn_base_2 (Utilities|Casting|CastToBP_VehicleAdvPawnBase _dockedvehicle))
          (Class|PrimitiveComponent|SetPhysicsAngularVelocityinDegrees (Variables|/Script/ChaosVehicles.WheeledVehiclePawn|GetMesh _asbp_vehicle_adv_pawn_base_2) "0, 0, 0" false "None")
          (Physics|SetPhysicsLinearVelocity (Variables|/Script/ChaosVehicles.WheeledVehiclePawn|GetMesh _asbp_vehicle_adv_pawn_base_2) "0, 0, 0" false "None"))))))

(fn ConstructionScript
  (bind _redcube (Variables|Default|GetRedCube))
  (Collision|SetCollisionProfileName _redcube "OverlapAllDynamic" true :!class /Script/Engine.PrimitiveComponent)
  (Collision|SetCollisionEnabled _redcube "QueryOnly"))