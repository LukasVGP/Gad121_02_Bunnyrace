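; BP_CurveSign is a curve sign actor that blinks and triggers a HUD warning when a vehicle overlaps it.
; Tick accumulates delta time and toggles the sign mesh's visibility each time the blink interval is reached.
; On overlap by a vehicle pawn, it calls ShowWarning on player 0's vehicle HUD, whichever vehicle entered.
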(event EventBeginPlay)

(event Collision|EventActorBeginOverlap
  (params (OtherActor :type Actor%20Object%20Reference))
  (Utilities|Casting|CastToBP_VehicleAdvPawnBase OtherActor)
  (bind _asbp_vehicle_adv_player_controller (Utilities|Casting|CastToBP_VehicleAdvPlayerController (Game|GetPlayerController 0)))
  (Default|ShowWarning (Variables|/Game/VehicleTemplate/Blueprints/BP_VehicleAdvPlayerController.BP_VehicleAdvPlayerController_C|GetVehicleHud _asbp_vehicle_adv_player_controller)))

(event EventTick
  (params (DeltaSeconds :type Float%20%28single-precision%29))
  (bind _output_get (Variables|Default|SetBlinkAccumulator (+ (Variables|Default|GetBlinkAccumulator) DeltaSeconds)))
  (if (>= _output_get (Variables|Default|GetBlinkInterval))
    (Rendering|ToggleVisibility (Variables|Default|GetSignMesh) false)
    (Variables|Default|SetBlinkAccumulator 0.0)))

(fn ConstructionScript)